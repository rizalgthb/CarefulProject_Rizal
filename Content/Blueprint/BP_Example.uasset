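; BP_Example is a small test Blueprint that simulates radiation exposure through on-screen debug messages.
; Pressing Tab calls RadiationFuction, which announces exposure, then raises RadiationScore in fixed steps with a while loop until it reaches the lethal threshold, printing each value.
; The loop completes within a single call, and death is only a printed message.
; The score is never reset, so later presses skip straight to the death message.
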(event `Key|Tab`
  (params (Key :type "Key Structure"))
  (:`Pressed`
    (`self.RadiationFuction`)))

(fn `RadiationFuction`
  (`KismetSystemLibrary.PrintString` "Player exposed to radiation." true true (struct :`G` 0.66 :`B` 1.0 :`A` 1.0) 10.0)
  (`KismetSystemLibrary.PrintString` (`KismetStringLibrary.Conv_IntToString` (`self.Radiation Score`)) true true (struct :`G` 0.66 :`B` 1.0 :`A` 1.0) 10.0)
  (while (< (`self.Radiation Score`) 100)
    (set `self.Radiation Score` (+ (`self.Radiation Score`) 25))
    (`KismetSystemLibrary.PrintString` (`KismetStringLibrary.Conv_IntToString` (`self.Radiation Score`)) true true (struct :`G` 0.66 :`B` 1.0 :`A` 1.0) 10.0))
  (`KismetSystemLibrary.PrintString` "Player died from radiation." true true (struct :`G` 0.66 :`B` 1.0 :`A` 1.0) 10.0))

(fn `UserConstructionScript`)